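; BP_Turret is an AI turret that attacks the player pawn when perceived and returns to pathing when it is forgotten.
; AI Perception events switch BP_TurretAIController between attacking and pathing states, writing the player to the blackboard Target key on sighting.
; Path spins the cube over time, and color events swap its material, showing white or grey at start depending on IsActive.
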(event OnPerceptionUpdated(AIPerception)
  (params (UpdatedActors :type Array%20of%20Actor%20Object%20References))
  (bind _returnvalue (Game|Player|GetPlayerPawn 0))
  (bind _self self)
  (bind _returnvalue_2 (AI|GetAIController _self))
  (for _array_element UpdatedActors
    (bind _sensed (CallFunction|CanSenseActor _array_element))
    (if _sensed
      (if (== _array_element _returnvalue)
        (bind _asbp_turret_aicontroller (Utilities|Casting|CastToBP_TurretAIController _returnvalue_2))
        (Default|SetStateasAttacking _asbp_turret_aicontroller)
        (AI|Components|Blackboard|SetValueasObject (Variables|/Script/AIModule.AIController|GetBlackboard _returnvalue_2) (Variables|Default|GetTarget) _returnvalue)))))

(event OnTargetPerceptionForgotten(AIPerception)
  (params (Actor :type Actor%20Object%20Reference))
  (if (== (Game|Player|GetPlayerPawn 0) Actor)
    (bind _asbp_turret_aicontroller (Utilities|Casting|CastToBP_TurretAIController (AI|GetAIController self)))
    (Default|SetStateasPathing _asbp_turret_aicontroller)))

(event Custom|ColorGrey
  (Rendering|Material|SetMaterial (Variables|Default|GetCube) 0 (Utilities|Array|Get(acopy) (Variables|Default|GetMaterial) 2)))

(event Custom|ColorWhite
  (Rendering|Material|SetMaterial (Variables|Default|GetCube) 0 (Utilities|Array|Get(acopy) (Variables|Default|GetMaterial))))

(event Custom|ColorRed
  (Rendering|Material|SetMaterial (Variables|Default|GetCube) 0 (Utilities|Array|Get(acopy) (Variables|Default|GetMaterial) 1)))

(event Custom|Path
  (Transformation|AddLocalRotation (Variables|Default|GetCube) (Math|Rotator|MakeRotator 0.0 0.0 (* (Variables|Default|GetRotationSpeed) (Utilities|Time|GetWorldDeltaSeconds))) false false))

(event EventBeginPlay
  (if (Variables|Default|GetIsActive)
    (CallFunction|ColorWhite)
    (else
      (CallFunction|ColorGrey))))

(fn ConstructionScript)

(fn CanSenseActor
  (params (Actor :type Actor%20Object%20Reference) (Sense :type Actor%20Object%20Reference))
  (bind _info (Class|AIPerceptionComponent|GetActorsPerception (Variables|Default|GetAIPerception) Actor))
  (for _array_element (.LastSensedStimuli (Utilities|Struct|BreakActorPerceptionBlueprintInfo _info))
    (return (.bSuccessfullySensed (Utilities|Struct|BreakAIStimulus _array_element)) _array_element)))

(fn HandleSensedSight
  (params (Actor :type Actor%20Object%20Reference))
  (bind _asbp_turret_aicontroller (Utilities|Casting|CastToBP_TurretAIController (AI|GetAIController self)))
  (Default|SetStateasAttacking _asbp_turret_aicontroller)
  (return))