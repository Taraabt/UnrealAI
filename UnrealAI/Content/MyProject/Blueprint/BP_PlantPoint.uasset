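; BP_PlantPoint is a plant spot whose sphere becomes ready a short time after activation.
; Activate shows the sphere with collision, then after a fixed delay sets IsReady, turns it green and broadcasts IsPlantReady with itself.
; DeActivate clears IsReady, hides the sphere, disables collision and turns it brown; BeginPlay also starts it hidden without collision.
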(event Custom|Activate
  (Rendering|SetVisibility (Variables|Default|GetSphere) true false)
  (Collision|SetCollisionEnabled (Variables|Default|GetSphere) "QueryAndPhysics")
  (Utilities|FlowControl|Delay 3.0)
  (Variables|Default|SetIs%20Ready true)
  (Rendering|Material|SetMaterial (Variables|Default|GetSphere) 0 "/Game/MyProject/Material/M_Green.M_Green")
  (Default|CallIsPlantReady self))

(event Custom|DeActivate
  (Variables|Default|SetIs%20Ready false)
  (Rendering|SetVisibility (Variables|Default|GetSphere) false false)
  (Collision|SetCollisionEnabled (Variables|Default|GetSphere) "NoCollision")
  (Rendering|Material|SetMaterial (Variables|Default|GetSphere) 0 "/Game/MyProject/Material/M_Brown.M_Brown"))

(event EventBeginPlay
  (Rendering|SetVisibility (Variables|Default|GetSphere) false false)
  (Collision|SetCollisionEnabled (Variables|Default|GetSphere) "NoCollision"))

(fn ConstructionScript)