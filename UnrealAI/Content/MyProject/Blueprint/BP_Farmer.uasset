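; BP_Farmer is an AI-controlled farmer that plants seeds at plant points and changes color through material swaps.
; Its Plant event clears HasSeed, then activates the BP_PlantPoint stored in its AI controller's Blackboard.
; Four color events set both mesh material slots from a Material array, with red applied at BeginPlay.
; Nothing in this graph calls Plant or the other colors.
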(event Custom|Plant
  (Variables|Default|SetHasSeed false)
  (bind _asbp_plant_point (Utilities|Casting|CastToBP_PlantPoint (AI|Components|Blackboard|GetValueasObject (Variables|/Script/AIModule.AIController|GetBlackboard (AI|GetAIController self)) (Variables|Default|GetPoint))))
  (Default|Activate _asbp_plant_point))

(event Custom|ColorPurple
  (for _index (range 0 1)
    (Rendering|Material|SetMaterial (Variables|Character|GetMesh) _index (Utilities|Array|Get(acopy) (Variables|Default|GetMaterial) 1))))

(event Custom|ColorRed
  (for _index (range 0 1)
    (Rendering|Material|SetMaterial (Variables|Character|GetMesh) _index (Utilities|Array|Get(acopy) (Variables|Default|GetMaterial)))))

(event Custom|ColorYellow
  (for _index (range 0 1)
    (Rendering|Material|SetMaterial (Variables|Character|GetMesh) _index (Utilities|Array|Get(acopy) (Variables|Default|GetMaterial) 3))))

(event Custom|ColorBlue
  (for _index (range 0 1)
    (Rendering|Material|SetMaterial (Variables|Character|GetMesh) _index (Utilities|Array|Get(acopy) (Variables|Default|GetMaterial) 2))))

(event EventBeginPlay
  (CallFunction|ColorRed))

(fn ConstructionScript)