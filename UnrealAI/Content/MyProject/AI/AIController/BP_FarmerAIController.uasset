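; BP_FarmerAIController is the AI controller for a farmer, running the BT_Farmer behavior tree on possess.
; On BeginPlay it gathers every BP_PlantPoint in the level, prints each name and binds an event to its IsPlantReady dispatcher.
; A SetPlant event writes the given plant to the PlantActor blackboard key for the behavior tree.
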(event Custom|SetPlant
  (params (Plant :type Actor%20Object%20Reference))
  (AI|Components|Blackboard|SetValueasObject (Variables|/Script/AIModule.AIController|GetBlackboard self) (Variables|Default|GetPlantActor) Plant))

(event EventBeginPlay
  (bind _outactors (Actor|GetAllActorsOfClass "/Game/MyProject/Blueprint/BP_PlantPoint.BP_PlantPoint_C"))
  (bind _output_get (Variables|Default|SetPlant%20Point _outactors))
  (for _array_element _output_get
    (bind _asbp_plant_point (Utilities|Casting|CastToBP_PlantPoint _array_element))
    (Development|PrintString (Utilities|GetDisplayName _asbp_plant_point))
    (EventDispatchers|BindEventtoIsPlantReady _asbp_plant_point (EventDispatchers|CreateEvent :!event Custom|SetPlant))))

(event EventPossess
  (params (PossessedPawn :type Pawn%20Object%20Reference))
  (AI|RunBehaviorTree "/Game/MyProject/AI/BT/BT_Farmer.BT_Farmer"))

(fn ConstructionScript)