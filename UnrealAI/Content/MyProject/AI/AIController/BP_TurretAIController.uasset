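; AI controller for the BP_Turret pawn that runs the turret's behavior tree.
; On BeginPlay it casts the controlled pawn to BP_Turret and, only if that turret is active, runs BT_Turret and sets the pathing state.
; Two events switch between attacking and pathing by writing an E_AITurretState value to the blackboard's state key.
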(event Custom|SetStateAsPathing
  (AI|Components|Blackboard|SetValueasEnum (AI|GetBlackboard 0) (Variables|Default|GetStateKeyName) (Utilities|Enum|LiteralenumE_AITurretState "NewEnumerator1")))

(event Custom|SetStateAsAttacking
  (AI|Components|Blackboard|SetValueasEnum (AI|GetBlackboard 0) (Variables|Default|GetStateKeyName) (Utilities|Enum|LiteralenumE_AITurretState "NewEnumerator0")))

(event EventBeginPlay
  (bind _asbp_turret (Utilities|Casting|CastToBP_Turret (Pawn|GetControlledPawn)))
  (if (Variables|/Game/MyProject/Blueprint/BP_Turret.BP_Turret_C|GetIsActive _asbp_turret)
    (AI|RunBehaviorTree "/Game/MyProject/AI/BT/BT_Turret.BT_Turret")
    (CallFunction|SetStateasPathing)))

(fn ConstructionScript)